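; BP_MixingTable is an interactable potion mixing table that opens its mixing interface when Initialize is called.
; It blends the player's view to the table, creates W_MixingTable with its BPMixingTableComponent, and switches to UI-only input with the cursor shown.
; The component's flags gate this: nothing opens when a potion is made but not available.
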(event `self.ReceiveBeginPlay`)

(event `self.Initialize`
  (bind _returnvalue (`GameplayStatics.GetPlayerController` 0))
  (bind _bp_mixingtablecomponent (`self.BP_MixingTableComponent`))
  (if (`MixingTableComponent.bPotionIsMade` _bp_mixingtablecomponent)
    (if (`MixingTableComponent.bPotionIsAvailable` _bp_mixingtablecomponent)
      (`PlayerController.SetViewTargetWithBlend` _returnvalue self 1.0 "VTBlend_Linear" 0.0 false :!label _label)
      (bind _returnvalue_2 (`|CreateWidget` "/Game/Widgets/MixingTable/W_MixingTable.W_MixingTable_C" _returnvalue (`self.BP_MixingTableComponent`)))
      (`UserWidget.AddToViewport` _returnvalue_2 0)
      (`WidgetBlueprintLibrary.SetInputMode_UIOnlyEx` _returnvalue _returnvalue_2 "DoNotLock" true)
      (set `PlayerController.bShowMouseCursor` true _returnvalue))
    (else
      (goto _label))))

(fn `UserConstructionScript`)