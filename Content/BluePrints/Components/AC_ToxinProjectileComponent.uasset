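; Actor component that gives the Poison Mutant character a toxin projectile attack with single and triple shot modes.
; On BeginPlay it caches the owning PoisonMutantCharacter, and FireShot routes to FireSingle or FireTriple by a bool.
; Both spawn BP_ToxinProjectile just in front of the owner's main camera along its rotation, with the owner set.
; The triple shot fans two extra projectiles out symmetrically in yaw.
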(event `self.ReceiveBeginPlay`
  (bind _aspoison_mutant_character (cast `PoisonMutantCharacter` (`self.GetOwner`)))
  (set `self.Player` _aspoison_mutant_character))

(event `FireShot`
  (params (SingleShot :type Boolean))
  (if SingleShot
    (`self.FireSingle`)
    (else
      (`self.Fire Triple`))))

(fn `Fire Triple`
  (bind _player (`self.Player`))
  (bind (_returnvalue _returnvalue2) (`self.Get FireLocation`))
  (`|SpawnActorFromClass` "/Game/BluePrints/PlayableCharacters/Toxin/BP_ToxinProjectile.BP_ToxinProjectile_C" (`KismetMathLibrary.MakeTransform` _returnvalue _returnvalue2) "Undefined" "OverrideRootScale" _player null)
  (bind _roll (.roll _returnvalue2))
  (bind _pitch (.pitch _returnvalue2))
  (bind _yaw (.yaw _returnvalue2))
  (`|SpawnActorFromClass` "/Game/BluePrints/PlayableCharacters/Toxin/BP_ToxinProjectile.BP_ToxinProjectile_C" (`KismetMathLibrary.MakeTransform` _returnvalue (`KismetMathLibrary.MakeRotator` _roll _pitch (+ _yaw 45.0))) "Undefined" "OverrideRootScale" _player null)
  (`|SpawnActorFromClass` "/Game/BluePrints/PlayableCharacters/Toxin/BP_ToxinProjectile.BP_ToxinProjectile_C" (`KismetMathLibrary.MakeTransform` _returnvalue (`KismetMathLibrary.MakeRotator` _roll _pitch (- _yaw 45.0))) "Undefined" "OverrideRootScale" _player null))

(fn `FireSingle`
  (bind (_returnvalue _returnvalue2) (`self.Get FireLocation`))
  (`|SpawnActorFromClass` "/Game/BluePrints/PlayableCharacters/Toxin/BP_ToxinProjectile.BP_ToxinProjectile_C" (`KismetMathLibrary.MakeTransform` _returnvalue _returnvalue2) "Undefined" "OverrideRootScale" (`self.Player`) null))

(fn `Get FireLocation`
  (returns (ReturnValue :type "Vector Structure") (ReturnValue2 :type "Rotator Structure"))
  (bind _maincamera (`PlayerCharacter.MainCamera` (`self.Player`)))
  (return (+ (`SceneComponent.K2_GetComponentLocation` _maincamera) (* (`SceneComponent.GetForwardVector` _maincamera) 10.0)) (`SceneComponent.K2_GetComponentRotation` _maincamera)))