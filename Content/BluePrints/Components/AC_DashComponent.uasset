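; Actor component that gives the player character a directional dash, suspending attacks while it runs.
; Initialize caches the player and movement component; Dash plays a section of the mutant attack montage, picked by dotting velocity with actor forward/right vectors, defaulting to backward.
; It adds an impulse along velocity scaled by DashStrength and restores CanAttack on blend out.
; A stationary dash only prints a "Crouch" placeholder.
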(event `Dash`
  (params (`Attack Component` :type "ComboAttackComponent Object Reference"))
  (bind _player (`self.Player`))
  (bind _charactermovement (`self.CharacterMovement`))
  (if (!= (`MovementComponent.Velocity` (`self.CharacterMovement`)) (0.0 0.0 0.0))
    (set `ComboAttackComponent.bCanAttack` false `Attack Component`)
    (set `ComboAttackComponent.bIsAttacking` false `Attack Component`)
    (`|PlayMontage` (`Character.Mesh` _player) (`PlayerCharacter.MutantAttackMontage` _player) 1.0 0.0 (`self.GetDashDirection`)
      (:`then`
        (`CharacterMovementComponent.AddImpulse` _charactermovement (* (* (`KismetMathLibrary.Normal` (`MovementComponent.Velocity` _charactermovement)) 300.0) (`self.Dash Strength`)) false))
      (:`OnBlendOut`
        (set `ComboAttackComponent.bCanAttack` true `Attack Component`)))
    (else
      ;[1 0.2726 0.2726] Crouch Component
      (`KismetSystemLibrary.PrintString` "Crouch"))))

(fn `GetDashDirection`
  (returns (Direction :type Name))
  (locals (Forward :type "Float (double-precision)" :default 0.0) (Right :type "Float (double-precision)" :default 0.0))
  (bind _returnvalue (`self.GetOwner`))
  (bind _forward (`local.Forward`))
  (bind _right (`local.Right`))
  (bind _returnvalue_2 (< _right -400.0))
  (bind _returnvalue_3 (< _forward -430.0))
  (set `local.Forward` (`KismetMathLibrary.Dot_VectorVector` (`MovementComponent.Velocity` (`self.CharacterMovement`)) (`Actor.GetActorForwardVector` _returnvalue)))
  (set `local.Right` (`KismetMathLibrary.Dot_VectorVector` (`MovementComponent.Velocity` (`self.CharacterMovement`)) (`Actor.GetActorRightVector` _returnvalue)))
  (`|ExecutionSequence`
    (:`then_0`
      (if (or (> _forward 430.0) _returnvalue_3)
        (return (select `bool` _returnvalue_3 :`false` "FrntDash" :`true` "BwrdDash" :!type "Name"))))
    (:`then_1`
      (if (or (> _right 400.0) _returnvalue_2)
        (return (select `bool` _returnvalue_2 :`false` "RightDash" :`true` "LeftDash" :!type "Name"))))
    (:`then_2`
      (return "BwrdDash"))))

(fn `Initialize`
  (params (PlayerCharacter :type "PlayerCharacter Object Reference"))
  (`/Engine/EditorBlueprintResources/StandardMacros.IsValid` PlayerCharacter
    (:`Is Valid`
      (bind _output_get (set `self.Player` PlayerCharacter))
      (set `self.CharacterMovement` (`Character.CharacterMovement` _output_get)))))