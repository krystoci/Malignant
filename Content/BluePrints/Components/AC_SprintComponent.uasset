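; Sprint component that switches a character's max walk speed between sprint and a fixed walk speed while managing stamina.
; Initialize receives the movement component and a CharacterStats struct, which supplies sprint speed and stamina values.
; Sprint toggles looping timers that drain stamina, stopping the sprint at zero, or refill it to base after a short delay.
; A Refilling flag prevents restarting an active refill; Tick is unused.
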(fn `DecreaseStamina`
  (bind _characterstats (`self.CharacterStats`))
  (bind _structout (setmembers `CharacterStats` :`StructRef` _characterstats :`CurrentStamina` (- (`.CurrentStamina` (break `CharacterStats` _characterstats)) 2.0)))
  (if (<= (`.CurrentStamina` (break `CharacterStats` _structout)) 0.0)
    (`self.Sprint` false)))

(fn `IncreaseStamina`
  (bind _characterstats (`self.CharacterStats`))
  (bind _structout (setmembers `CharacterStats` :`StructRef` _characterstats :`CurrentStamina` (+ (`.CurrentStamina` (break `CharacterStats` _characterstats)) 2.0)))
  (bind (_basehealth _basedefense _baseattack _basestamina _basesprintspeed _currenthealth _currentdefense _currentattack _currentstamina) (break `CharacterStats` _structout))
  (if (>= _currentstamina _basestamina)
    (setmembers `CharacterStats` :`StructRef` _structout :`CurrentStamina` _basestamina)
    (`KismetSystemLibrary.K2_ClearAndInvalidateTimerHandle` (`self.IncreaseHandle`))
    (set `self.Refilling` false)))

(fn `Initialize`
  (params (`Character Movement Component` :type "CharacterMovementComponent Object Reference") (`Character Stats` :type "CharacterStats Structure"))
  (set `self.CharacterMovement` `Character Movement Component`)
  (set `self.CharacterStats` `Character Stats`))

(fn `Sprint`
  (params (StartSprint :type Boolean))
  (bind _charactermovement (`self.CharacterMovement`))
  (if StartSprint
    (set `self.Refilling` false)
    (`KismetSystemLibrary.K2_ClearAndInvalidateTimerHandle` (`self.IncreaseHandle`))
    (set `CharacterMovementComponent.MaxWalkSpeed` (`.CurrentSprintSpeed` (break `CharacterStats` (`self.CharacterStats`))) _charactermovement)
    (bind _returnvalue (`KismetSystemLibrary.K2_SetTimer` null "DecreaseStamina" 0.1 true))
    (set `self.DecreaseHandle` _returnvalue)
    (else
      (`KismetSystemLibrary.K2_ClearAndInvalidateTimerHandle` (`self.DecreaseHandle`))
      (if (not (`self.Refilling`))
        (set `CharacterMovementComponent.MaxWalkSpeed` 600.0 _charactermovement)
        (bind _returnvalue_2 (`KismetSystemLibrary.K2_SetTimer` null "IncreaseStamina" 0.05 true 2.0))
        (set `self.IncreaseHandle` _returnvalue_2)
        (set `self.Refilling` true)))))