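; Actor component for the Bone Blade Mutant character that fires bone projectiles, alternating between right and left blade sockets.
; FireBone disables attacking and aims at the actor hit by a forward sphere trace, falling back to main camera rotation.
; It caches socket location and montage section before playing the attack montage.
; The montage's FireBone notify spawns the projectile, and attacking re-enables only when the montage completes.
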(event `self.ReceiveBeginPlay`
  (bind _asbp_bone_blade_mutant_character (cast `/Game/BluePrints/PlayableCharacters/BoneBlade/BP_BoneBladeMutantCharacter` (`self.GetOwner`)))
  (set `self.BoneBladeCharacter` _asbp_bone_blade_mutant_character))

(event `FireBone`
  (params (SkeletalMesh :type "SkeletalMeshComponent Object Reference"))
  (bind _bonebladecharacter (`self.BoneBladeCharacter`))
  (bind _returnvalue (`Actor.K2_GetActorLocation` _bonebladecharacter))
  (bind _returnvalue_2 (`Actor.GetActorForwardVector` _bonebladecharacter))
  (`/Engine/EditorBlueprintResources/StandardMacros.IsValid` _bonebladecharacter
    (:`Is Valid`
      (set `ComboAttackComponent.bCanAttack` false (`MutantCharacter.AttackComponent` _bonebladecharacter))
      (bind _outhit (`KismetSystemLibrary.SphereTraceSingle` (+ _returnvalue (* _returnvalue_2 600.0)) (+ _returnvalue (* _returnvalue_2 5000.0)) 400.0 "TraceTypeQuery3"))
      (bind (_bblockinghit _binitialoverlap _time _distance _location _impactpoint _normal _impactnormal _physmat _hitactor) (`GameplayStatics.BreakHitResult` _outhit))
      (if _bblockinghit
        (bind _returnvalue_3 (`KismetMathLibrary.FindLookAtRotation` _returnvalue (`Actor.K2_GetActorLocation` _hitactor)))
        (`KismetSystemLibrary.PrintString` (`KismetStringLibrary.Conv_RotatorToString` _returnvalue_3))
        (set `self.FireRotation` _returnvalue_3)
        (else
          (set `self.FireRotation` (`SceneComponent.K2_GetComponentRotation` (`PlayerCharacter.MainCamera` (`self.BoneBladeCharacter`))))))
      (`self.GetFireLocation`)
      (bind _notifyname (`|PlayMontage` SkeletalMesh "/Game/BluePrints/PlayableCharacters/BoneBlade/Animations/AM_BoneBlades_Attack.AM_BoneBlades_Attack" 1.0 0.0 (`self.Starting Section`))
        (:`OnCompleted`
          (set `ComboAttackComponent.bCanAttack` true (`MutantCharacter.AttackComponent` (`self.BoneBladeCharacter`))))
        (:`OnNotifyBegin`
          (if (== _notifyname "FireBone")
            (`|SpawnActorFromClass` "/Game/BluePrints/PlayableCharacters/BoneBlade/BP_BoneProjectile.BP_BoneProjectile_C" (`KismetMathLibrary.MakeTransform` (`self.FireLocation`) (`self.FireRotation`)) "AlwaysSpawn" "OverrideRootScale" null (`self.BoneBladeCharacter`))))))))

(fn `GetFireLocation`
  (if (`self.isRight`)
    (set `self.FireLocation` (`SceneComponent.GetSocketLocation` (`Character.Mesh` (`self.BoneBladeCharacter`)) "R_BoneBladeSocketStart"))
    (set `self.Starting Section` "ShootShardRight")
    (set `self.isRight` false)
    (else
      (set `self.FireLocation` (`SceneComponent.GetSocketLocation` (`Character.Mesh` (`self.BoneBladeCharacter`)) "L_BoneBladeSocketStart"))
      (set `self.Starting Section` "ShootShardLeft")
      (set `self.isRight` true))))