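; Actor component that lets the PoisonMutantCharacter climb walls whose physical material has SurfaceType3.
; TryWallClimb multi-sphere-traces around the player and, on a match, switches to Flying movement, pitches the camera and faces the wall.
; While climbing, Tick re-traces, turning actor and controller into the impact normal and snapping location to the hit.
; Losing the surface restores Falling and resets actor and camera rotation.
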(event `self.ReceiveTick`
  (params (DeltaSeconds :type "Float (single-precision)"))
  (bind _player (`self.Player`))
  (bind _returnvalue (`Actor.K2_GetActorLocation` _player))
  (if (`self.IsClimbing`)
    (bind _outhit (`KismetSystemLibrary.SphereTraceSingle` _returnvalue _returnvalue 100.0 "TraceTypeQuery1" false (`|MakeArray` _player :!type "Actor Object Reference")))
    (bind (_bblockinghit _binitialoverlap _time _distance _location _impactpoint _normal _impactnormal _physmat) (`GameplayStatics.BreakHitResult` _outhit))
    (if _bblockinghit
      (if (`|EnumEquality` (`PhysicalMaterial.SurfaceType` _physmat) "SurfaceType3")
        (`self.SetActorClimbRotation` _impactnormal)
        (`Actor.K2_SetActorLocation` (`self.Player`) _location false false)
        (else
          (`self.StopWallClimb` :!label _label)))
      (else
        (goto _label)))))

(event `self.ReceiveBeginPlay`
  (bind _aspoison_mutant_character (cast `PoisonMutantCharacter` (`self.GetOwner`)))
  (set `self.Player` _aspoison_mutant_character))

(event `TryWallClimb`
  (bind _returnvalue (`Actor.K2_GetActorLocation` (`self.Player`)))
  (if (not (`self.IsClimbing`))
    (`/Engine/EditorBlueprintResources/StandardMacros.IsValid` (`self.Player`)
      (:`Is Valid`
        (bind _outhits (`KismetSystemLibrary.SphereTraceMulti` :`Start` _returnvalue :`End` _returnvalue :`Radius` 100.0 :`TraceChannel` "TraceTypeQuery1" :`DrawDebugType` "ForDuration"))
        (for _array_element _outhits
          (bind (_bblockinghit _binitialoverlap _time _distance _location _impactpoint _normal _impactnormal _physmat) (`GameplayStatics.BreakHitResult` _array_element))
          (if _bblockinghit
            (if (`|EnumEquality` (`PhysicalMaterial.SurfaceType` _physmat) "SurfaceType3")
              (`self.StartWallClimb` _array_element)
              (break))))))))

(event `StartWallClimb`
  (params (HitResult :type "HitResult Structure"))
  (bind _player (`self.Player`))
  (`CharacterMovementComponent.SetMovementMode` (`Character.CharacterMovement` (`self.Player`)) "MOVE_Flying" 0)
  (set `PoisonMutantCharacter.isWallClimbing` true _player)
  (`SceneComponent.K2_SetRelativeRotation` (`PlayerCharacter.MainCamera` _player) (`KismetMathLibrary.MakeRotator` 0.0 90.0) false false)
  (`self.SetActorClimbRotation` (`.ImpactNormal` (`GameplayStatics.BreakHitResult` HitResult)))
  (set `self.IsClimbing` true))

(event `StopWallClimb`
  (bind _player (`self.Player`))
  (if (`self.IsClimbing`)
    (`CharacterMovementComponent.SetMovementMode` (`Character.CharacterMovement` _player) "MOVE_Falling" 0)
    (set `self.IsClimbing` false)
    (set `PoisonMutantCharacter.isWallClimbing` false _player)
    (`Actor.K2_SetActorRotation` :`self` _player)
    (`SceneComponent.K2_SetRelativeRotation` :`self` (`PlayerCharacter.MainCamera` _player))))

(fn `SetActorClimbRotation`
  (params (`Impact Vector` :type "Vector Structure"))
  (bind _player (`self.Player`))
  (bind _returnvalue_roll (`KismetMathLibrary.BreakRotator` (`Actor.K2_GetActorRotation` _player)))
  (bind (_returnvalue_roll_2 _returnvalue_pitch _returnvalue_yaw) (`KismetMathLibrary.BreakRotator` (`KismetMathLibrary.Conv_VectorToRotator` (`KismetMathLibrary.NegateVector` `Impact Vector`))))
  (`Actor.K2_SetActorRotation` _player (`KismetMathLibrary.MakeRotator` _returnvalue_roll _returnvalue_pitch _returnvalue_yaw) false)
  (`Controller.SetControlRotation` (`Pawn.GetController` _player) (`KismetMathLibrary.MakeRotator` _returnvalue_roll _returnvalue_pitch _returnvalue_yaw)))