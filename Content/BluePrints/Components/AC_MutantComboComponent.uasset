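; Actor component for mutant combo attacks that plays montage sections by name at a given speed.
; Section "4" plays the BoneBladeSpecial montage only if the owner is a BoneBladeMutantCharacter; other sections use AttackMontage.
; In both cases, montage completion calls FinishAttack and a notify begin opens the combo frame through ToggleComboFrame.
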(event `self.PlayAnimationMontage`
  (params (Section :type Name) (Speed :type "Float (single-precision)"))
  (if (== Section "4")
    (cast `BoneBladeMutantCharacter` (`self.GetOwner`))
    (`|PlayMontage` (`self.CharacterMeshComponent`) (`self.BoneBladeSpecial`) Speed 0.0 "4"
      (:`OnCompleted`
        (`self.FinishAttack`))
      (:`OnNotifyBegin`
        (`self.ToggleComboFrame` true)))
    (else
      (`|PlayMontage` (`self.CharacterMeshComponent`) (`self.AttackMontage`) Speed 0.0 Section
        (:`OnCompleted`
          (`self.FinishAttack`))
        (:`OnNotifyBegin`
          (`self.ToggleComboFrame` true))))))