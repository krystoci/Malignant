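; BP_TestDummy is a damageable test dummy that loses health when something overlaps its skeletal mesh.
; Overlaps from BP_BoneBladeMutantCharacter deal heavier damage than any other actor, through the OnRecieveDamage event.
; Each hit plays a timeline that drives the Color Scale parameter on a dynamic material created at BeginPlay.
; When health runs out, it also disables capsule collision and switches the mesh to physics simulation.
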(event `self.ReceiveBeginPlay`
  (bind _returnvalue (`PrimitiveComponent.CreateDynamicMaterialInstance` (`self.SkeletalMesh`) 0 "/Game/BluePrints/M_DummyMaterial.M_DummyMaterial" "None"))
  (set `self.BaseMaterial` _returnvalue))

(event `On Recieve Damage`
  (params (Damage :type Integer))
  (bind _output_get (set `self.Health` (- (`self.Health`) Damage)))
  (if (<= _output_get 0)
    (`PrimitiveComponent.SetCollisionEnabled` (`self.Capsule`) "NoCollision")
    (`PrimitiveComponent.SetSimulatePhysics` (`self.SkeletalMesh`) true)
    (bind (_direction _newtrack_0) (`Timeline|Timeline` :!via `PlayFromStart` :!label _label)
      (:`Update`
        (`MaterialInstanceDynamic.SetScalarParameterValue` (`self.BaseMaterial`) "Color Scale" _newtrack_0)))
    (else
      (goto _label :!via `PlayFromStart`))))

(event `self.SkeletalMesh.OnComponentBeginOverlap`
  (params (OverlappedComponent :type "PrimitiveComponent Object Reference") (OtherActor :type "Actor Object Reference") (OtherComp :type "PrimitiveComponent Object Reference") (OtherBodyIndex :type Integer) (bFromSweep :type Boolean) (SweepResult :type "HitResult Structure (by ref)"))
  (cast `/Game/Mutants/Blueprints/BoneBlade/BP_BoneBladeMutantCharacter` OtherActor
    (:`then`
      (`self.On Recieve Damage` 20))
    (:`CastFailed`
      (`self.On Recieve Damage` 2))))

(fn `UserConstructionScript`)