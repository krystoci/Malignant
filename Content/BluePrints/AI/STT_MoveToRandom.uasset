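; State Tree task that sends the AI-controlled actor to a random navigable point around its current location.
; On entering the state, it picks a point within a fixed radius, keeps the actor's current height, starts a MoveTo and prints the request result.
; Tick only records the actor's location and keeps returning Running, so the task never completes by itself.
; Exiting the state stops the controller's movement.
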(event `self.ReceiveExitState`
  (params (Transition :type "StateTreeTransitionResult Structure (by ref)"))
  (`Controller.StopMovement` (`AIBlueprintHelperLibrary.GetAIController` (`self.Actor`))))

(fn `ReceiveEnterState`
  (params (Transition :type "StateTreeTransitionResult Structure (by ref)"))
  (returns (ReturnValue :type "EStateTreeRunStatus Enum"))
  (bind _actor (`self.Actor`))
  (bind (_returnvalue_x _returnvalue_y _returnvalue_z) (`KismetMathLibrary.BreakVector` (`Actor.K2_GetActorLocation` _actor)))
  (bind _randomlocation (`NavigationSystemV1.K2_GetRandomLocationInNavigableRadius` (`KismetMathLibrary.MakeVector` _returnvalue_x _returnvalue_y _returnvalue_z) 1000.0 null null))
  (bind _output_get (set `self.Move to Location` (`KismetMathLibrary.MakeVector` (.x _randomlocation) (.y _randomlocation) _returnvalue_z)))
  (bind _returnvalue (`AIController.MoveToLocation` (`AIBlueprintHelperLibrary.GetAIController` _actor) _output_get 10.0 false true false true null true))
  (`KismetSystemLibrary.PrintString` (`|GetEnumeratorNameAsString` _returnvalue))
  (return "Running"))

(fn `ReceiveTick`
  (params (DeltaTime :type "Float (single-precision)"))
  (returns (ReturnValue :type "EStateTreeRunStatus Enum"))
  (set `self.Actor Location` (`Actor.K2_GetActorLocation` (`self.Actor`)))
  (return "Running"))