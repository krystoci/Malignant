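; BP_MoveToPlayer is a StateTree task that makes an AI character chase the player.
; Entering the state sets the character's max walk speed to a fixed value.
; Each tick re-issues a MoveToActor request through the AI controller with a small acceptance radius and prints the request result for debugging.
; The task always returns Running, so it never finishes on its own.
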(fn `ReceiveEnterState`
  (params (Transition :type "StateTreeTransitionResult Structure (by ref)"))
  (returns (ReturnValue :type "EStateTreeRunStatus Enum"))
  (set `CharacterMovementComponent.MaxWalkSpeed` 300.0 (`Character.CharacterMovement` (`self.Character`)))
  (return "Running"))

(fn `ReceiveTick`
  (params (DeltaTime :type "Float (single-precision)"))
  (returns (ReturnValue :type "EStateTreeRunStatus Enum"))
  (bind _returnvalue (`AIController.MoveToActor` (`AIBlueprintHelperLibrary.GetAIController` (`self.Character`)) (`self.Player`) 15.0 false true true null true))
  (`KismetSystemLibrary.PrintString` (`|GetEnumeratorNameAsString` _returnvalue))
  (return "Running"))