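; BP_BoneBladeEnemy is an AI enemy Blueprint that detects the player by sight.
; When its PawnSensing component sees a PlayerCharacter, it sends a PawnSensed event to its StateTree and fires PawnFound with that character.
; Other pawns are ignored, and the Blueprint has no active BeginPlay, overlap or Tick logic of its own.
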(event `self.PawnSensing.OnSeePawn`
  (params (Pawn :type "Pawn Object Reference"))
  (bind _asplayer_character (cast `PlayerCharacter` Pawn))
  (`StateTreeComponent.SendStateTreeEvent` (`self.StateTree`) (make `StateTreeEvent` (struct :`TagName` "PawnSensed")))
  (`self.PawnFound` _asplayer_character))

(fn `UserConstructionScript`
  (`parent.UserConstructionScript`))