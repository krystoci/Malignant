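; BP_Door is a damageable door that the player barricades with carried chairs or a desk.
; Tick polls for R while the player is inside the Box overlap, then reveals pre-placed furniture meshes, sets an extra-health buffer, destroys the carried actor and sets walk speed.
; AnyDamage drains that buffer first; once empty, damage hides the first chair and reduces door health, swapping to a destroyed mesh before destroying the actor at zero.
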(event `self.ReceiveAnyDamage`
  (params (Damage :type "Float (single-precision)") (DamageType :type "DamageType Object Reference") (InstigatedBy :type "Controller Object Reference") (DamageCauser :type "Actor Object Reference"))
  ;[1 1 1] Test for the door damage
  (`self.DamageDoor` Damage))

(event `self.ReceiveTick`
  (params (DeltaSeconds :type "Float (single-precision)"))
  (bind _asbp_last_stand_character (cast `/Game/BluePrints/PlayableCharacters/BP_LastStandCharacter` (`Controller.K2_GetPawn` (`GameplayStatics.GetPlayerController` 0)) :!pure true))
  ;[1 1 1] System for repair door with objects and add extra health to the door
  ;;[0 0.2331 1] Event Tick
  (`|ExecutionSequence`
    (:`then_0`
      ;;[1 1 1] Repair the door with object
      (`self.RepairDoorWithObject` (`/Game/BluePrints/RepairSystem/BP_Chair.IsChair` (`/Game/BluePrints/PlayableCharacters/BP_LastStandCharacter.HeldChair` _asbp_last_stand_character)) (`/Game/BluePrints/RepairSystem/BP_Desk.IsDesk` (`/Game/BluePrints/PlayableCharacters/BP_LastStandCharacter.HeldTable` _asbp_last_stand_character)) (`/Game/BluePrints/PlayableCharacters/BP_LastStandCharacter.ActorAttach` _asbp_last_stand_character)))))

(event `self.ReceiveBeginPlay`
  (bind _asbp_last_stand_character (cast `/Game/BluePrints/PlayableCharacters/BP_LastStandCharacter` (`Controller.K2_GetPawn` (`GameplayStatics.GetPlayerController` 0)) :!pure true))
  ;[1 1 1] System for repair door with objects and add extra health to the door
  ;;[0 0.1803 1] Begin Play
  (set `/Game/BluePrints/PlayableCharacters/BP_LastStandCharacter.Door` self _asbp_last_stand_character)
  (set `self.HeldChair` (`/Game/BluePrints/PlayableCharacters/BP_LastStandCharacter.HeldChair` _asbp_last_stand_character))
  (set `self.HeldDesk` (`/Game/BluePrints/PlayableCharacters/BP_LastStandCharacter.HeldTable` _asbp_last_stand_character))
  (bind _asbp_mallignant_player_controller (cast `/Game/BluePrints/Controllers/BP_MallignantPlayerController` (`GameplayStatics.GetPlayerController` 0)))
  (set `self.PCMalignant` _asbp_mallignant_player_controller))

(event `self.Box.OnComponentBeginOverlap`
  (params (OverlappedComponent :type "PrimitiveComponent Object Reference") (OtherActor :type "Actor Object Reference") (OtherComp :type "PrimitiveComponent Object Reference") (OtherBodyIndex :type Integer) (bFromSweep :type Boolean) (SweepResult :type "HitResult Structure (by ref)"))
  ;[1 1 1] System for repair door with objects and add extra health to the door
  ;;[1 1 1] Check if the player is inside the collision box
  (cast `/Game/BluePrints/PlayableCharacters/BP_LastStandCharacter` OtherActor)
  (set `self.PlayerInBounds` true))

(event `self.Box.OnComponentEndOverlap`
  (params (OverlappedComponent :type "PrimitiveComponent Object Reference") (OtherActor :type "Actor Object Reference") (OtherComp :type "PrimitiveComponent Object Reference") (OtherBodyIndex :type Integer))
  ;[1 1 1] System for repair door with objects and add extra health to the door
  ;;[1 1 1] Check if the player is inside the collision box
  (cast `/Game/BluePrints/PlayableCharacters/BP_LastStandCharacter` OtherActor)
  (set `self.PlayerInBounds` false))

(fn `DamageDoor`
  (params (DamageTaken :type "Float (double-precision)"))
  (bind _chairmodel (`self.ChairModel`))
  (bind _door (`self.Door`))
  (set `self.ExtraHealthByObject` (`KismetMathLibrary.FClamp` (- (`self.ExtraHealthByObject`) DamageTaken)))
  (if (== (`self.ExtraHealthByObject`) 0.0)
    (`SceneComponent.SetVisibility` _chairmodel false false)
    (`PrimitiveComponent.SetCollisionEnabled` _chairmodel "NoCollision")
    (set `self.Health` (`KismetMathLibrary.FClamp` (- (`self.Health`) DamageTaken)))
    (if (<= (`self.Health`) 0.7)
      (`StaticMeshComponent.SetStaticMesh` _door "/Game/Assets/Door/SM_Door_Destroyed.SM_Door_Destroyed")
      (`SceneComponent.K2_SetRelativeRotation` _door (struct :`Pitch` -1e-06 :`Yaw` 359.999999 :`Roll` -359.999999) false false)
      (`SceneComponent.K2_SetRelativeLocation` _door (-78.437183 -7.330169 115.079583) false false)
      (`SceneComponent.SetRelativeScale3D` _door (0.465967 0.522193 0.478673))
      (if (== (`self.Health`) 0.0)
        (`self.K2_DestroyActor`)))))

(fn `RepairDoorWithObject`
  (params (IsChair :type Boolean) (IsDesk :type Boolean) (AttachActor :type "Actor Object Reference"))
  (bind _chairmodel1 (`self.ChairModel1`))
  (bind _chairmodel (`self.ChairModel`))
  (bind _desk (`self.Desk`))
  (if (and (`SceneComponent.IsVisible` (`self.Desk`)) (`SceneComponent.IsVisible` (`self.ChairModel`)) (`SceneComponent.IsVisible` (`self.ChairModel1`)))
    (`SceneComponent.SetVisibility` (`self.ChairModel2`) true false)
    (`SceneComponent.SetVisibility` (`self.ChairModel3`) true false)
    (`SceneComponent.SetVisibility` (`self.ChairModel`) false false)
    (`SceneComponent.SetVisibility` (`self.ChairModel1`) false false)
    (elif (and IsChair (`self.PlayerInBounds`) (`PlayerController.IsInputKeyDown` (`GameplayStatics.GetPlayerController` 0) "R"))
      (if (and (`SceneComponent.IsVisible` (`self.ChairModel`)) (`self.PlayerInBounds`))
        (`SceneComponent.SetVisibility` _chairmodel1 true false)
        (`PrimitiveComponent.SetCollisionEnabled` _chairmodel1 "QueryAndPhysics")
        (set `self.ExtraHealthByObject` (+ (`/Game/BluePrints/RepairSystem/BP_Chair.Health` (`self.HeldChair`)) 0.2))
        (set `self.PlayerInBounds` false)
        (`self.K2_DestroyActor` AttachActor)
        (set `CharacterMovementComponent.MaxWalkSpeed` 600.0 (`Character.CharacterMovement` (`GameplayStatics.GetPlayerCharacter` 0)))
        (else
          (`SceneComponent.SetVisibility` _chairmodel true false)
          (`PrimitiveComponent.SetCollisionEnabled` _chairmodel "QueryAndPhysics")
          (set `self.ExtraHealthByObject` (+ (`/Game/BluePrints/RepairSystem/BP_Chair.Health` (`self.HeldChair`)) 0.2))
          (set `self.PlayerInBounds` false)
          (`self.K2_DestroyActor` AttachActor)
          (set `CharacterMovementComponent.MaxWalkSpeed` 600.0 (`Character.CharacterMovement` (`GameplayStatics.GetPlayerCharacter` 0)))))
      (elif (and IsDesk (`self.PlayerInBounds`) (`PlayerController.IsInputKeyDown` (`GameplayStatics.GetPlayerController` 0) "R"))
        (`SceneComponent.SetVisibility` _desk true false)
        (`PrimitiveComponent.SetCollisionEnabled` _desk "QueryAndPhysics")
        (set `self.ExtraHealthByObject` (+ (`/Game/BluePrints/RepairSystem/BP_Desk.Health` (`self.HeldDesk`)) 0.5))
        (set `self.PlayerInBounds` false)
        (`self.K2_DestroyActor` AttachActor)
        (set `CharacterMovementComponent.MaxWalkSpeed` 600.0 (`Character.CharacterMovement` (`GameplayStatics.GetPlayerCharacter` 0)))))))

(fn `UserConstructionScript`)