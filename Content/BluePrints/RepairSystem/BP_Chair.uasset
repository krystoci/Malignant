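; BP_Chair is a repair system chair that the player takes hold of by interacting with it.
; Interact casts the player character to BP_LastStandCharacter, registers the chair as HeldChair, flags an object as taken and sets a fixed walk speed.
; A DoOnce gate blocks repeat interactions until ResetTakeChair resets it.
; The file contains no attachment or placement logic, only this state handoff to the character.
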(event `/Game/BluePrints/Interfaces/BPI_Interact.Interact`
  (`/Engine/EditorBlueprintResources/StandardMacros.DoOnce` false :!label _label
    (:`Completed`
      (bind _asbp_last_stand_character (cast `/Game/BluePrints/PlayableCharacters/BP_LastStandCharacter` (`GameplayStatics.GetPlayerCharacter` 0)))
      (set `/Game/BluePrints/PlayableCharacters/BP_LastStandCharacter.HeldChair` self _asbp_last_stand_character)
      (set `/Game/BluePrints/PlayableCharacters/BP_LastStandCharacter.IsObjectTacked` true _asbp_last_stand_character)
      (set `self.IsChair` true)
      (set `CharacterMovementComponent.MaxWalkSpeed` 400.0 (`Character.CharacterMovement` (`GameplayStatics.GetPlayerCharacter` 0))))))

(event `ResetTakeChair`
  (goto _label :!via `Reset`))

(fn `UserConstructionScript`)