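; BP_TestDummy is a test enemy that takes damage, flashes through its material and can be decapitated.
; Damage lowers Health and plays a timeline driving the dynamic material's Color Scale; at zero health the capsule loses collision and the mesh ragdolls.
; Box overlap hides the neck bone, self-applies heavy damage and spawns a BP_BoneBladeHead once at the neck socket.
; Overlapping projectiles pass their velocity, plus lift, to that head as an impulse.
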(event `self.ReceiveBeginPlay`
  (bind _returnvalue (`PrimitiveComponent.CreateDynamicMaterialInstance` (`self.SkeletalMesh`) 0 "/Game/Materials/M_DummyMaterial.M_DummyMaterial" "None"))
  (set `self.BaseMaterial` _returnvalue))

(event `self.ReceiveAnyDamage`
  (params (Damage :type "Float (single-precision)") (DamageType :type "DamageType Object Reference") (InstigatedBy :type "Controller Object Reference") (DamageCauser :type "Actor Object Reference"))
  (bind _output_get (set `self.Health` (- (`self.Health`) Damage)))
  (if (<= _output_get 0.0)
    (`PrimitiveComponent.SetCollisionEnabled` (`self.Capsule`) "NoCollision")
    (`PrimitiveComponent.SetSimulatePhysics` (`self.SkeletalMesh`) true)
    (bind (_direction _newtrack_0) (`Timeline|Timeline` :!via `PlayFromStart` :!label _label)
      (:`Update`
        (`MaterialInstanceDynamic.SetScalarParameterValue` (`self.BaseMaterial`) "Color Scale" _newtrack_0)))
    (else
      (goto _label :!via `PlayFromStart`))))

(event `self.SkeletalMesh.OnComponentBeginOverlap`
  (params (OverlappedComponent :type "PrimitiveComponent Object Reference") (OtherActor :type "Actor Object Reference") (OtherComp :type "PrimitiveComponent Object Reference") (OtherBodyIndex :type Integer) (bFromSweep :type Boolean) (SweepResult :type "HitResult Structure (by ref)"))
  (cast `/Game/BluePrints/PlayableCharacters/BoneBlade/BP_BoneBladeMutantCharacter` OtherActor))

(event `self.Box.OnComponentBeginOverlap`
  (params (OverlappedComponent :type "PrimitiveComponent Object Reference") (OtherActor :type "Actor Object Reference") (OtherComp :type "PrimitiveComponent Object Reference") (OtherBodyIndex :type Integer) (bFromSweep :type Boolean) (SweepResult :type "HitResult Structure (by ref)"))
  (bind _returnvalue (`self.GetComponentByClass` OtherActor "/Script/Engine.ProjectileMovementComponent"))
  (bind _returnvalue_roll (`KismetMathLibrary.BreakRotator` (`self.K2_GetActorRotation`)))
  (bind _skeletalmesh (`self.SkeletalMesh`))
  (bind _returnvalue_2 (`SceneComponent.GetSocketTransform` _skeletalmesh "neck" "RTS_World"))
  (`SkinnedMeshComponent.HideBoneByName` _skeletalmesh "neck" "PBO_None")
  (`GameplayStatics.ApplyDamage` self 100.0)
  (`/Engine/EditorBlueprintResources/StandardMacros.DoOnce` false
    (:`Completed`
      (bind _returnvalue_3 (`|SpawnActorFromClass` "/Game/BluePrints/NPCs/Enemies/TestDummy/BP_BoneBladeHead.BP_BoneBladeHead_C" (`KismetMathLibrary.MakeTransform` (.location _returnvalue_2) (`KismetMathLibrary.MakeRotator` _returnvalue_roll (.pitch (.rotation _returnvalue_2)) (.yaw (.rotation _returnvalue_2))) (.scale _returnvalue_2)) "AlwaysSpawn" "OverrideRootScale" null null))
      (`/Engine/EditorBlueprintResources/StandardMacros.IsValid` _returnvalue
        (:`Is Valid`
          (`PrimitiveComponent.AddImpulse` (`/Game/BluePrints/NPCs/Enemies/TestDummy/BP_BoneBladeHead.StaticMesh` _returnvalue_3) (* (+ (`MovementComponent.Velocity` _returnvalue) (0.0 0.0 100.0)) 10.0) "None" false))))))

(fn `UserConstructionScript`)