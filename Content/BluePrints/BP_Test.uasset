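; Test Blueprint that handles entering and leaving interaction with an in-game PC menu.
; UsePC flags interaction, enables collision on the passed PCMenu actor and eases the player's view over to it.
; While interacting, Tick polls a key to re-possess the player character, restore game-only input and movement, hide the cursor and clear the flag.
; Exiting leaves the menu's collision enabled.
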(event `UsePC`
  (params (PCMenu :type "/Game/BluePrints/BP_Test Object Reference"))
  (set `self.IsInteracting?` true)
  (`self.SetActorEnableCollision` PCMenu true)
  (`PlayerController.SetViewTargetWithBlend` (`GameplayStatics.GetPlayerController` 0) PCMenu 1.0 "VTBlend_EaseIn" 1.0 false))

(event `self.ReceiveTick`
  (params (DeltaSeconds :type "Float (single-precision)"))
  (bind _returnvalue (`GameplayStatics.GetPlayerController` 0))
  (if (`self.IsInteracting?`)
    (if (`PlayerController.IsInputKeyDown` _returnvalue "One")
      (`Controller.Possess` _returnvalue (`GameplayStatics.GetPlayerCharacter` 0))
      (`WidgetBlueprintLibrary.SetInputMode_GameOnly` _returnvalue)
      (`Controller.ResetIgnoreMoveInput` _returnvalue)
      (set `PlayerController.bShowMouseCursor` false _returnvalue)
      (set `self.IsInteracting?` false))))

(fn `UserConstructionScript`)