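; BP_LastStandCharacter is a playable character Blueprint that can pick up repair objects and test damage on doors.
; Interact line-traces forward from RayCastLocation, sends InteractMessage to actors tagged RepairObject, then snaps them to the ObjectTakedLook component.
; The F key is a test input that sphere-traces forward and applies a small amount of damage to the hit actor.
; Both traces use the Visibility channel with debug drawing enabled.
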(event `Key|F`
  (params (Key :type "Key Structure"))
  (bind _raycastlocation (`self.RayCastLocation`))
  (bind _returnvalue (`SceneComponent.K2_GetComponentLocation` _raycastlocation))
  ;[1 1 1] Test for apply damage to doors
  (:`Pressed`
    (bind (_outhit _returnvalue_2) (`KismetSystemLibrary.SphereTraceSingle` :`Start` _returnvalue :`End` (+ _returnvalue (* (`SceneComponent.GetForwardVector` _raycastlocation) 200.0)) :`TraceChannel` "TraceTypeQuery1" :`DrawDebugType` "ForDuration"))
    (if _returnvalue_2
      (`GameplayStatics.ApplyDamage` (`.HitActor` (`GameplayStatics.BreakHitResult` _outhit)) 0.2 null self))))

(event `InputAction|Interact`
  (params (Key :type "Key Structure"))
  (bind _raycastlocation (`self.RayCastLocation`))
  (bind _returnvalue (`SceneComponent.K2_GetComponentLocation` _raycastlocation))
  ;[1 1 1] Interact with objects to repair/add extra health to doors
  (:`Pressed`
    (bind (_outhit _returnvalue_2) (`KismetSystemLibrary.LineTraceSingle` :`Start` _returnvalue :`End` (+ _returnvalue (* (`SceneComponent.GetForwardVector` _raycastlocation) 150.0)) :`TraceChannel` "TraceTypeQuery1" :`DrawDebugType` "Persistent"))
    (if _returnvalue_2
      (bind (_bblockinghit _binitialoverlap _time _distance _location _impactpoint _normal _impactnormal _physmat _hitactor) (`GameplayStatics.BreakHitResult` _outhit))
      (if (`self.ActorHasTag` _hitactor "RepairObject")
        (message `/Game/BluePrints/Interfaces/BPI_Interact.Interact` _hitactor)
        (bind _output_get (set `self.ActorAttach` _hitactor))
        (`self.K2_AttachToComponent` _output_get (`self.ObjectTakedLook`) "None" "SnapToTarget" "SnapToTarget" "SnapToTarget" true)))))

(fn `UserConstructionScript`)