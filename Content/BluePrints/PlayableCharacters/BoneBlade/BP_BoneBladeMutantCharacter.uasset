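; Playable Bone Blade mutant character with melee blade attacks, a bone projectile, a sharpen montage and a charged AOE.
; Attacks run timed socket-to-socket traces per blade, damaging each actor once per blade and slicing procedural meshes along the swing plane.
; Holding Ability3 slows movement and builds radius; release expands a timeline-driven sphere that currently only prints overlapped enemies.
; It also attaches the camera and equipped items to mesh sockets.
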(event `AttackStart`
  (bind _mesh (`self.Mesh`))
  (set `self.RightBoneStart` (`SceneComponent.GetSocketLocation` _mesh "R_BoneBladeSocketStart"))
  (set `self.LeftBoneStart` (`SceneComponent.GetSocketLocation` _mesh "L_BoneBladeSocketStart"))
  (`self.AttackTrace`)
  (bind _returnvalue (`KismetSystemLibrary.K2_SetTimer` null "AttackTrace" 0.005 true))
  (set `self.AttackHandle` _returnvalue))

(event `AttackEnd`
  (`KismetSystemLibrary.K2_ClearAndInvalidateTimerHandle` (`self.AttackHandle`))
  (`KismetArrayLibrary.Array_Clear` (`self.ActorsHitRight`))
  (`KismetArrayLibrary.Array_Clear` (`self.ActorsHitLeft`)))

(event `InputAction|Ability1`
  (params (Key :type "Key Structure"))
  (:`Pressed`
    (`/Game/BluePrints/Components/AC_BoneProjectileComponent.FireBone` (`self.BP_BoneProjectileComponent`))))

(event `self.ReceiveBeginPlay`
  (`SceneComponent.K2_AttachToComponent` (`self.MainCamera`) (`self.Mesh`) "cameraSocket" "SnapToTarget" "SnapToTarget" "KeepRelative" false))

(event `InputAction|Ability2`
  (params (Key :type "Key Structure"))
  (:`Pressed`
    (`self.Sharpen Bones`)))

(event `InputAction|Ability3`
  (params (Key :type "Key Structure"))
  (:`Pressed`
    (if (not (`self.AOETriggered`))
      (set `CharacterMovementComponent.MaxWalkSpeed` 50.0 (`self.CharacterMovement`))
      (bind _returnvalue (`KismetSystemLibrary.K2_SetTimer` null "AddCharge" 0.2 true))
      (set `self.AOEChargeHandle` _returnvalue)))
  (:`Released`
    (set `CharacterMovementComponent.MaxWalkSpeed` 600.0 (`self.CharacterMovement`))
    (`KismetSystemLibrary.K2_ClearAndInvalidateTimerHandle` (`self.AOEChargeHandle`))
    (if (> (`self.AOEPower`) 0)
      (set `self.AOEPower` 0)
      (`self.BoneAOE`))))

(event `BoneAOE`
  (bind _overlapping_actors (`self.Overlapping Actors`))
  (if (not (`self.AOETriggered`))
    (set `self.AOETriggered` true)
    (bind _returnvalue (`AddComponent|NODE_AddSphereComponent-0`))
    (bind (_direction _newtrack_0) (`Timeline|SphereTrace` :!via `PlayFromStart`)
      (:`Update`
        (`SceneComponent.SetWorldScale3D` _returnvalue (`KismetMathLibrary.VLerp` (0.0 0.0 0.0) (`self.AOE Radius`) _newtrack_0))
        (`KismetSystemLibrary.DrawDebugSphere` (`self.K2_GetActorLocation`) (`SphereComponent.GetScaledSphereRadius` _returnvalue) 12 (struct :`R` 0.030518 :`G` 1.0 :`A` 1.0) 0.1 0.5)
        (for _array_element (`PrimitiveComponent.GetOverlappingActors` _returnvalue "/Script/Malignant.BaseEnemy")
          (`BlueprintSetLibrary.Set_Add` (`self.Overlapping Actors`) _array_element)))
      (:`Finished`
        (`ActorComponent.K2_DestroyComponent` _returnvalue)
        (if (not (`BlueprintSetLibrary.Set_IsEmpty` _overlapping_actors))
          (bind _result (`BlueprintSetLibrary.Set_ToArray` _overlapping_actors))
          (for _array_element_2 _result
            (`KismetSystemLibrary.PrintString` (`KismetSystemLibrary.GetDisplayName` _array_element_2)))
          (`BlueprintSetLibrary.Set_Clear` (`self.Overlapping Actors`)))
        (set `self.AOE Radius` (0.0 0.0 0.0))
        (set `self.AOETriggered` false)
        (`KismetSystemLibrary.PrintString` "Reset")))))

(event `self.EquipItem`
  (params (NewItem :type "ItemPickupBase Object Reference"))
  (`/Engine/EditorBlueprintResources/StandardMacros.IsValid` NewItem
    (:`Is Valid`
      (set `self.EquippedItem` NewItem)
      (`self.SetActorEnableCollision` NewItem false)
      (`self.K2_AttachToComponent` NewItem (`self.Mesh`) "R_HandSocket" "SnapToTarget" "KeepRelative" "KeepWorld" false))))

(fn `AddCharge`
  (if (< (`self.AOEPower`) 10)
    (`/Engine/EditorBlueprintResources/StandardMacros.IncrementInt` (`self.AOEPower`)
      (:`  `
        (bind _output_get (set `self.AOE Radius` (+ (`self.AOE Radius`) (2.0 2.0 2.0))))
        (`KismetSystemLibrary.PrintString` (`KismetStringLibrary.Conv_VectorToString` _output_get))))))

(fn `AttackTrace`
  (bind _mesh (`self.Mesh`))
  (bind _mesh_2 (`self.Mesh`))
  (switch `name` (`ComboAttackComponent.AttackSection` (`self.AttackComponent`))
    (:`Default`
      (`|ExecutionSequence`
        (:`then_0`
          (bind (_outhit _returnvalue) (`KismetSystemLibrary.LineTraceSingle` :`Start` (`SceneComponent.GetSocketLocation` _mesh_2 "R_BoneBladeSocketStart") :`End` (`SceneComponent.GetSocketLocation` _mesh_2 "R_BoneBladeSocketEnd") :`TraceChannel` "TraceTypeQuery3" :`DrawDebugType` "ForDuration" :`DrawTime` 1.0 :!label _label))
          (if _returnvalue
            (`self.HandleHit` _outhit true)))
        (:`then_1`
          (bind (_outhit_2 _returnvalue_2) (`KismetSystemLibrary.LineTraceSingle` :`Start` (`SceneComponent.GetSocketLocation` _mesh "L_BoneBladeSocketStart") :`End` (`SceneComponent.GetSocketLocation` _mesh "L_BoneBladeSocketEnd") :`TraceChannel` "TraceTypeQuery3" :`DrawDebugType` "ForDuration" :`DrawTime` 1.0 :!label _label_2))
          (if _returnvalue_2
            (`self.HandleHit` _outhit_2)))))
    (:`0`
      (goto _label))
    (:`1`
      (goto _label_2))))

(fn `HandleHit`
  (params (BlockingHit :type "HitResult Structure") (`RightBlade?` :type Boolean))
  (locals (PlaneNormal :type "Vector Structure") (HitLocation :type "Vector Structure" :default (0.0 0.0 0.0)))
  (bind (_bblockinghit _binitialoverlap _time _distance _location _impactpoint _normal _impactnormal _physmat _hitactor _hitcomponent) (`GameplayStatics.BreakHitResult` BlockingHit))
  (bind _mesh (`self.Mesh`))
  (bind _actorshitleft (`self.ActorsHitLeft`))
  (bind _mesh_2 (`self.Mesh`))
  (bind _actorshitright (`self.ActorsHitRight`))
  (bind _returnvalue (`SceneComponent.GetSocketLocation` _mesh_2 "R_BoneBladeSocketEnd"))
  (bind _returnvalue_2 (`SceneComponent.GetSocketLocation` _mesh "L_BoneBladeSocketEnd"))
  (set `local.HitLocation` _location)
  (if `RightBlade?`
    (bind _returnvalue_3 (`KismetArrayLibrary.Array_AddUnique` _actorshitright _hitactor))
    (if (`KismetArrayLibrary.Array_IsValidIndex` _actorshitright _returnvalue_3)
      (`|ExecutionSequence` :!label _label
        (:`then_0`
          (`GameplayStatics.ApplyDamage` _hitactor 20.0))
        (:`then_1`
          (if (`local.RightBlade?`)
            (set `local.PlaneNormal` (`KismetMathLibrary.Cross_VectorVector` (- (`self.RightBoneStart`) _returnvalue) (- (`SceneComponent.GetSocketLocation` _mesh_2 "R_BoneBladeSocketStart") _returnvalue)))
            (else
              (set `local.PlaneNormal` (`KismetMathLibrary.Cross_VectorVector` (- (`self.LeftBoneStart`) _returnvalue_2) (- (`SceneComponent.GetSocketLocation` _mesh "L_BoneBladeSocketStart") _returnvalue_2)))))
          (bind _asprocedural_mesh_component (cast `ProceduralMeshComponent` _hitcomponent))
          (bind _outotherhalfprocmesh (`KismetProceduralMeshLibrary.SliceProceduralMesh` _asprocedural_mesh_component (`local.HitLocation`) (`local.PlaneNormal`) true "CreateNewSectionForCap" "/Engine/EngineMeshes/BackgroundMaterial.BackgroundMaterial"))
          (`PrimitiveComponent.SetSimulatePhysics` _outotherhalfprocmesh true)
          (`PrimitiveComponent.AddImpulse` _outotherhalfprocmesh (0.0 0.0 100.0) "None" true))))
    (else
      (bind _returnvalue_4 (`KismetArrayLibrary.Array_AddUnique` _actorshitleft _hitactor))
      (if (`KismetArrayLibrary.Array_IsValidIndex` _actorshitleft _returnvalue_4)
        (goto _label)))))

(fn `Sharpen Bones`
  (`self.PlayAnimMontage` "/Game/BluePrints/PlayableCharacters/BoneBlade/Animations/AM_BoneBlades_Attack.AM_BoneBlades_Attack" 1.0 "SharpenBladeBoth"))

(fn `UserConstructionScript`)