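; GS_MalignantGameState is a game state Blueprint that spawns and possesses the player's character for a given class.
; SpawnPlayer looks the class up in MutantMap and spawns the mapped actor at the current pawn's location.
; Player controller 0 possesses the new actor, and its BP_MallignantPlayerController PlayerPawn reference is updated.
; The step that destroys the previous pawn is disconnected, so this event leaves that pawn in place.
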(event `self.SpawnPlayer`
  (params (CharacterClass :type "EMutantState Enum" :default "Human"))
  (bind _returnvalue (`GameplayStatics.GetPlayerController` 0))
  (bind (_value _returnvalue_2) (`BlueprintMapLibrary.Map_Find` (`self.MutantMap`) CharacterClass))
  (if _returnvalue_2
    (bind _output_get (set `self.SpawnLocation` (`self.K2_GetActorLocation` (`GameplayStatics.GetPlayerPawn` 0))))
    (bind _returnvalue_3 (`|SpawnActorFromClass` _value (`KismetMathLibrary.MakeTransform` _output_get) "Undefined" "OverrideRootScale" null null))
    (`Controller.Possess` _returnvalue _returnvalue_3)
    (set `/Game/BluePrints/Controllers/BP_MallignantPlayerController.PlayerPawn` _returnvalue_3 (cast `/Game/BluePrints/Controllers/BP_MallignantPlayerController` _returnvalue :!pure true))))

(fn `UserConstructionScript`)