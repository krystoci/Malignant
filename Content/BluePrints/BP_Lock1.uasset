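; BP_Lock1 is a timing-minigame chest lock that takes the camera on overlap and spins a needle over randomly rotated targets.
; Tick runs a short line trace for "Correct"-tagged components and polls left mouse to stop the needle and judge it.
; Boolean flags step through three stages, swapping check meshes, collision boxes and bulb materials.
; A miss resets and returns control; final success drops the lock, opens the chest and animates the acquired object.
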(event `PlayNeedle`
  (bind _faceplate_base (`self.Faceplate_Base`))
  (bind (_direction _newtrack_0) (`Timeline|RotateNeedle` :!label _label)
    (:`Update`
      (`SceneComponent.K2_SetRelativeRotation` (`self.Lock_Needle`) (`KismetMathLibrary.MakeRotator` 0.0 _newtrack_0) false false)
      (`/Engine/EditorBlueprintResources/StandardMacros.DoOnce` false :!label _label_2
        (:`Completed`
          (`SceneComponent.K2_SetRelativeRotation` (`self.Check_3`) (`KismetMathLibrary.MakeRotator` -90.0 (`KismetMathLibrary.RandomFloatInRange` 0.0 360.0)) false false)
          (`KismetSystemLibrary.Delay` 0.6)
          (`PrimitiveComponent.SetMaterial` _faceplate_base 0 "/Game/Assets/Lock/Materials/M_FacePlate_Red.M_FacePlate_Red")
          (`KismetSystemLibrary.Delay` 0.2)
          (`PrimitiveComponent.SetMaterial` _faceplate_base 0 "/Game/Assets/Lock/Materials/M_Faceplate.M_Faceplate")
          (`KismetSystemLibrary.Delay` 0.2)
          (`PrimitiveComponent.SetMaterial` _faceplate_base 0 "/Game/Assets/Lock/Materials/M_FacePlate_Red.M_FacePlate_Red")
          (`KismetSystemLibrary.Delay` 0.6)
          (`SceneComponent.SetVisibility` _faceplate_base false false)
          (`self.PlayNeedle`)
          (bind _returnvalue (`GameplayStatics.SpawnSoundAtLocation` "/Game/Audio/Sounds/ClockTask_TimerTicking_Cue.ClockTask_TimerTicking_Cue" (`SceneComponent.RelativeLocation` (`self.Lock_Needle`)) (struct) 1.0 1.0 0.0 null null))
          (set `self.TimingAudio` _returnvalue)
          (`SceneComponent.SetVisibility` (`self.Check_3`) true false)
          (`PrimitiveComponent.SetCollisionEnabled` (`self.Box8`) "NoCollision")
          (`PrimitiveComponent.SetCollisionEnabled` (`self.Box9`) "NoCollision")
          (`PrimitiveComponent.SetCollisionEnabled` (`self.Box2`) "NoCollision")
          (`PrimitiveComponent.SetCollisionEnabled` (`self.Box6`) "NoCollision")
          (`PrimitiveComponent.SetCollisionEnabled` (`self.Box7`) "NoCollision"))))
    (:`Finished`
      (`self.Bucle`))))

(event `self.Collision_Interact.OnComponentBeginOverlap`
  (params (OverlappedComponent :type "PrimitiveComponent Object Reference") (OtherActor :type "Actor Object Reference") (OtherComp :type "PrimitiveComponent Object Reference") (OtherBodyIndex :type Integer) (bFromSweep :type Boolean) (SweepResult :type "HitResult Structure (by ref)"))
  (`Controller.SetIgnoreMoveInput` (`GameplayStatics.GetPlayerController` 0) false)
  (set `self.IsInteracting?` true)
  (cast `PlayerCharacter` OtherActor)
  (`PlayerController.SetViewTargetWithBlend` (`GameplayStatics.GetPlayerController` 0) self 0.5 "VTBlend_EaseIn" 0.5 false)
  (goto _label_2))

(event `Bucle`
  (goto _label :!via `PlayFromStart`))

(event `StopNeedle`
  (goto _label :!via `Stop`))

(event `ResetButtonClick`
  (bind (_direction _newtrack_0 _newtrack_1) (`Timeline|PressButtonClick` :!via `Reverse` :!label _label_3)
    (:`Update`
      (`SceneComponent.K2_SetRelativeLocation` (`self.PressButton1`) (`KismetMathLibrary.MakeVector` _newtrack_0 (.y _newtrack_1) (.z _newtrack_1)) false false))
    (:`Finished`
      (`self.ResetButtonClick`)
      (`/Engine/EditorBlueprintResources/StandardMacros.DoOnce` false :!label _label_4
        (:`Completed`
          (`GameplayStatics.PlaySoundAtLocation` "/Game/Audio/Sounds/ClockTask_Clicker_1.ClockTask_Clicker_1" (`SceneComponent.RelativeLocation` (`self.Lock_Needle`)) (struct) 1.0 1.0 0.0 null null null null))))))

(event `NextStage`
  (bind _returnvalue (`GameplayStatics.GetPlayerController` 0))
  (bind _check_1 (`self.Check_1`))
  (bind _lock_top (`self.Lock_Top`))
  (bind _chesttop (`self.ChestTop`))
  (bind _faceplate_base (`self.Faceplate_Base`))
  (bind _faceplate_base_2 (`self.Faceplate_Base`))
  (bind _check_2 (`self.Check_2`))
  (bind (_relativelocation_x _relativelocation_y) (`KismetMathLibrary.BreakVector` (`SceneComponent.RelativeLocation` _lock_top)))
  (if (`self.IsInteracting?`) :!label _label_5
    (if (`PlayerController.IsInputKeyDown` (`GameplayStatics.GetPlayerController` 0) "LeftMouseButton")
      (`|ExecutionSequence`
        (:`then_0`
          (`self.StopNeedle`)
          (goto _label_3))
        (:`then_1`
          (`KismetSystemLibrary.Delay` 0.5)
          (if (`self.IsCorrect?`)
            (`KismetSystemLibrary.PrintString` "Correct!" true true (struct :`G` 1.0 :`B` 0.005564 :`A` 1.0))
            (`|ExecutionSequence`
              (:`then_0`
                (`self.PlayNeedle`)
                (`GameplayStatics.PlaySound2D` "/Game/Audio/Sounds/ClockTask_Change_1.ClockTask_Change_1" 1.0 1.0 0.0 null null))
              (:`then_1`
                (`SceneComponent.SetVisibility` (`self.Check_3`) false false)
                (`PrimitiveComponent.SetCollisionEnabled` (`self.Box`) "NoCollision")
                (`PrimitiveComponent.SetCollisionEnabled` (`self.Box5`) "NoCollision")
                (`PrimitiveComponent.SetCollisionEnabled` (`self.Box4`) "NoCollision")
                (`PrimitiveComponent.SetCollisionEnabled` (`self.Box2`) "QueryAndPhysics")
                (`PrimitiveComponent.SetCollisionEnabled` (`self.Box6`) "QueryAndPhysics")
                (`PrimitiveComponent.SetCollisionEnabled` (`self.Box7`) "QueryAndPhysics")
                (`SceneComponent.SetVisibility` _check_2 true false)
                (`SceneComponent.K2_SetRelativeRotation` _check_2 (`KismetMathLibrary.MakeRotator` -90.0 (`KismetMathLibrary.RandomFloatInRange` 0.0 360.0)) false false)
                (set `self.Correct2` true))
              (:`then_2`
                (if (`self.Next?`)
                  (`SceneComponent.SetVisibility` (`self.Check_2`) false false)
                  (`PrimitiveComponent.SetCollisionEnabled` (`self.Box2`) "NoCollision")
                  (`PrimitiveComponent.SetCollisionEnabled` (`self.Box6`) "NoCollision")
                  (`PrimitiveComponent.SetCollisionEnabled` (`self.Box7`) "NoCollision")
                  (`PrimitiveComponent.SetCollisionEnabled` (`self.Box8`) "QueryAndPhysics")
                  (`PrimitiveComponent.SetCollisionEnabled` (`self.Box9`) "QueryAndPhysics")
                  (`SceneComponent.SetVisibility` _check_1 true false)
                  (`SceneComponent.K2_SetRelativeRotation` _check_1 (`KismetMathLibrary.MakeRotator` -90.0 (`KismetMathLibrary.RandomFloatInRange` 0.0 360.0)) false false)
                  (set `self.Correct2` true)
                  (set `self.Correct1` false)
                  (`PrimitiveComponent.SetMaterial` (`self.Lock_Bulb_2`) 0 "/Game/Materials/M_Yelow.M_Yelow")
                  (if (`self.Next2?`)
                    (set `self.Correct3` true)
                    (set `self.Stop` true)
                    (`AudioComponent.Stop` (`self.TimingAudio`))
                    (`GameplayStatics.PlaySound2D` "/Game/Audio/Sounds/ClockTask_Unlock_1.ClockTask_Unlock_1" 1.0 1.0 0.0 null null)
                    (`PrimitiveComponent.SetMaterial` (`self.Lock_Bulb_3`) 0 "/Game/Materials/M_Yelow.M_Yelow")
                    (`SceneComponent.SetVisibility` _faceplate_base_2 true false)
                    (`PrimitiveComponent.SetMaterial` _faceplate_base_2 0 "/Game/Assets/Lock/Materials/M_FacePlate_Green.M_FacePlate_Green")
                    (`KismetSystemLibrary.Delay` 0.2)
                    (`PrimitiveComponent.SetMaterial` _faceplate_base_2 0 "/Game/Assets/Lock/Materials/M_Faceplate.M_Faceplate")
                    (`KismetSystemLibrary.Delay` 0.2)
                    (`PrimitiveComponent.SetMaterial` _faceplate_base_2 0 "/Game/Assets/Lock/Materials/M_FacePlate_Green.M_FacePlate_Green")
                    (`SceneComponent.SetVisibility` (`self.Check_3`) false false)
                    (`SceneComponent.SetVisibility` (`self.Check_1`) false false)
                    (`SceneComponent.SetVisibility` (`self.Check_2`) false false)
                    (bind (_direction _newtrack_0) (`Timeline|MoveLockTop`)
                      (:`Update`
                        (`SceneComponent.K2_SetRelativeLocation` _lock_top (`KismetMathLibrary.MakeVector` _relativelocation_x _relativelocation_y _newtrack_0) false false)
                        (`PrimitiveComponent.SetCollisionEnabled` (`self.Box1`) "NoCollision")
                        (`PrimitiveComponent.SetCollisionEnabled` (`self.Box`) "NoCollision")
                        (`PrimitiveComponent.SetCollisionEnabled` (`self.Box4`) "NoCollision")
                        (`PrimitiveComponent.SetCollisionEnabled` (`self.Box5`) "NoCollision")
                        (`PrimitiveComponent.SetCollisionEnabled` (`self.Box2`) "NoCollision")
                        (`PrimitiveComponent.SetCollisionEnabled` (`self.Box6`) "NoCollision")
                        (`PrimitiveComponent.SetCollisionEnabled` (`self.Box9`) "NoCollision")
                        (`PrimitiveComponent.SetCollisionEnabled` (`self.Box7`) "NoCollision")
                        (`PrimitiveComponent.SetCollisionEnabled` (`self.Box8`) "NoCollision")
                        (`KismetSystemLibrary.Delay` 1.0)
                        (`Controller.Possess` _returnvalue (`GameplayStatics.GetPlayerCharacter` 0))
                        (`Controller.ResetIgnoreMoveInput` _returnvalue)
                        (`PrimitiveComponent.SetSimulatePhysics` (`self.Lock_Body`) true)
                        (`ActorComponent.K2_DestroyComponent` (`self.Collision_Interact`))
                        (bind (_direction_2 _newtrack_0_2) (`Timeline|RotateTopChest`)
                          (:`Update`
                            (`SceneComponent.K2_SetRelativeRotation` _chesttop (`KismetMathLibrary.MakeRotator` _newtrack_0_2) false false)
                            (`SceneComponent.K2_SetRelativeLocation` _chesttop (-2.580782 106.810127 133.265793) false false)
                            (`KismetSystemLibrary.Delay` 1.0)
                            (bind (_direction_3 _objectup) (`Timeline|ObjectUP`)
                              (:`Update`
                                (`SceneComponent.K2_SetRelativeLocation` (`self.ObjectAdquired`) (`KismetMathLibrary.MakeVector` 0.0 0.0 _objectup) false false))
                              (:`Finished`
                                (bind (_direction_4 _objectup_2) (`Timeline|ObjectUP/Down` :!label _label_6)
                                  (:`Update`
                                    (`SceneComponent.K2_SetRelativeLocation` (`self.ObjectAdquired`) (`KismetMathLibrary.MakeVector` 0.0 0.0 _objectup_2) false false)
                                    (`KismetSystemLibrary.Delay` 1.3)
                                    (`self.ReverseObject`))
                                  (:`Finished`
                                    (`self.PlayAgain`))))))))))
                  (else
                    (set `self.Correct1` true)
                    (`PrimitiveComponent.SetMaterial` (`self.Lock_Bulb_1`) 0 "/Game/Materials/M_Yelow.M_Yelow")))))
            (else
              (`KismetSystemLibrary.PrintString` "Incorrect!" true true (struct :`R` 1.0 :`G` 0.959716 :`A` 1.0))
              (`Controller.Possess` (`GameplayStatics.GetPlayerController` 0) (`GameplayStatics.GetPlayerCharacter` 0))
              (`SceneComponent.SetVisibility` (`self.Check_1`) false false)
              (`SceneComponent.SetVisibility` (`self.Check_2`) false false)
              (`SceneComponent.SetVisibility` (`self.Check_3`) false false)
              (set `self.Stop` false)
              (`|ExecutionSequence`
                (:`then_0`
                  (goto _label_2 :!via `Reset`))
                (:`then_1`
                  (`GameplayStatics.PlaySound2D` "/Game/Audio/Sounds/ClockTask_Fail_1.ClockTask_Fail_1" 1.0 1.0 0.0 null null)
                  (`AudioComponent.Stop` (`self.TimingAudio`)))
                (:`then_2`
                  (`PrimitiveComponent.SetCollisionEnabled` (`self.Box`) "QueryAndPhysics")
                  (`PrimitiveComponent.SetCollisionEnabled` (`self.Box5`) "QueryAndPhysics")
                  (`PrimitiveComponent.SetCollisionEnabled` (`self.Box4`) "QueryAndPhysics")
                  (`PrimitiveComponent.SetCollisionEnabled` (`self.Box2`) "NoCollision")
                  (`PrimitiveComponent.SetCollisionEnabled` (`self.Box6`) "NoCollision")
                  (`PrimitiveComponent.SetCollisionEnabled` (`self.Box7`) "NoCollision")
                  (`PrimitiveComponent.SetCollisionEnabled` (`self.Box8`) "NoCollision")
                  (`PrimitiveComponent.SetCollisionEnabled` (`self.Box9`) "NoCollision"))
                (:`then_3`
                  (`PrimitiveComponent.SetMaterial` (`self.Lock_Bulb_1`) 0 "/Game/Assets/Lock/Materials/M_Lock.M_Lock")
                  (`PrimitiveComponent.SetMaterial` (`self.Lock_Bulb_2`) 0 "/Game/Assets/Lock/Materials/M_Lock.M_Lock")
                  (`PrimitiveComponent.SetMaterial` (`self.Lock_Bulb_3`) 0 "/Game/Assets/Lock/Materials/M_Lock.M_Lock")
                  (`SceneComponent.SetVisibility` _faceplate_base true false)
                  (`PrimitiveComponent.SetMaterial` _faceplate_base 0 "/Game/Assets/Lock/Materials/M_Faceplate.M_Faceplate"))
                (:`then_4`
                  (set `self.Correct1` false)
                  (set `self.Correct2` false)
                  (set `self.Correct3` false)
                  (set `self.Next?` false)
                  (set `self.Next2?` false))))))
        (:`then_2`
          (`self.ResetSoundClick`))))))

(event `self.ReceiveTick`
  (params (DeltaSeconds :type "Float (single-precision)"))
  (`|ExecutionSequence`
    (:`then_0`
      (if (`self.Stop`)
        (`self.StopNeedle`)
        (elif (`self.Correct1`)
          (`self.NextStage`)
          (set `self.Next?` true)
          (elif (`self.Correct2`)
            (`self.NextStage`)
            (set `self.Next2?` true)
            (else
              (goto _label_5))))))
    (:`then_1`
      (`self.NeedleTrace`))))

(event `PlayAgain`
  (goto _label_6))

(event `ResetSoundClick`
  (goto _label_4 :!via `Reset`))

(event `ReverseObject`
  (goto _label_6 :!via `Reverse`))

(fn `NeedleTrace`
  (bind _box1 (`self.Box1`))
  (bind _returnvalue (`SceneComponent.K2_GetComponentLocation` _box1))
  (bind (_outhit _returnvalue_2) (`KismetSystemLibrary.LineTraceSingle` :`Start` _returnvalue :`End` (+ _returnvalue (* (`KismetMathLibrary.GetForwardVector` (`SceneComponent.K2_GetComponentRotation` _box1)) 5.0)) :`TraceChannel` "TraceTypeQuery1" :`bTraceComplex` true :`bIgnoreSelf` false))
  (if _returnvalue_2
    (if (`ActorComponent.ComponentHasTag` (`.HitComponent` (`GameplayStatics.BreakHitResult` _outhit)) "Correct")
      (set `self.IsCorrect?` true)
      (else
        (set `self.IsCorrect?` false)))
    (else
      (set `self.IsCorrect?` false))))

(fn `UserConstructionScript`)