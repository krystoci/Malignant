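; BP_BottlePickup is a bottle item that shows a text prompt while the player is nearby.
; DisplayBounds overlap events store the overlapping PlayerCharacter and show TextRender, then hide it and clear the reference on exit.
; While a player is stored, Tick rotates the Scene component to face that player's MainCamera, billboarding it toward the view.
; No pickup or collection logic is implemented in this Blueprint.
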(event `self.ReceiveTick`
  (params (DeltaSeconds :type "Float (single-precision)"))
  (bind _overlappingactor (`self.OverlappingActor`))
  (bind _scene (`self.Scene`))
  (`/Engine/EditorBlueprintResources/StandardMacros.IsValid` _overlappingactor
    (:`Is Valid`
      (`SceneComponent.K2_SetWorldRotation` _scene (`KismetMathLibrary.FindLookAtRotation` (`SceneComponent.K2_GetComponentLocation` _scene) (`SceneComponent.K2_GetComponentLocation` (`PlayerCharacter.MainCamera` _overlappingactor))) false false))))

(event `self.DisplayBounds.OnComponentBeginOverlap`
  (params (OverlappedComponent :type "PrimitiveComponent Object Reference") (OtherActor :type "Actor Object Reference") (OtherComp :type "PrimitiveComponent Object Reference") (OtherBodyIndex :type Integer) (bFromSweep :type Boolean) (SweepResult :type "HitResult Structure (by ref)"))
  (bind _asplayer_character (cast `PlayerCharacter` OtherActor))
  (set `self.OverlappingActor` _asplayer_character)
  (`SceneComponent.SetVisibility` (`self.TextRender`) true false))

(event `self.DisplayBounds.OnComponentEndOverlap`
  (params (OverlappedComponent :type "PrimitiveComponent Object Reference") (OtherActor :type "Actor Object Reference") (OtherComp :type "PrimitiveComponent Object Reference") (OtherBodyIndex :type Integer))
  (cast `PlayerCharacter` OtherActor)
  (`SceneComponent.SetVisibility` (`self.TextRender`) false false)
  (set `self.OverlappingActor` null))

(fn `UserConstructionScript`)