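; BP_MallignantPlayerController is a player controller that routes attack input to the controlled character.
; It caches the pawn as a PlayerCharacter on BeginPlay and on possession.
; LightAttack and HeavyAttack presses cast that pawn to MutantCharacter and call the matching attack, with only the light attack checking validity first.
; Widget interaction nodes for simulated left-mouse press and release are present but disconnected.
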(event `self.ReceiveBeginPlay`
  (bind _asplayer_character (cast `PlayerCharacter` (`self.K2_GetPawn`)))
  (set `self.PlayerPawn` _asplayer_character))

(event `self.ReceivePossess`
  (params (PossessedPawn :type "Pawn Object Reference"))
  (bind _asplayer_character (cast `PlayerCharacter` PossessedPawn))
  (set `self.PlayerPawn` _asplayer_character))

(event `Key|LeftMouseButton`
  (params (Key :type "Key Structure"))
  ;[0 0.2182 1] Interact Widget
)

(event `InputAction|LightAttack`
  (params (Key :type "Key Structure"))
  (bind _playerpawn (`self.PlayerPawn`))
  (:`Pressed`
    (`/Engine/EditorBlueprintResources/StandardMacros.IsValid` _playerpawn
      (:`Is Valid`
        (bind _asmutant_character (cast `MutantCharacter` _playerpawn))
        (`MutantCharacter.LightAttack` _asmutant_character)))))

(event `InputAction|HeavyAttack`
  (params (Key :type "Key Structure"))
  (:`Pressed`
    (bind _asmutant_character (cast `MutantCharacter` (`self.PlayerPawn`)))
    (`MutantCharacter.HeavyAttack` _asmutant_character)))

(fn `UserConstructionScript`)