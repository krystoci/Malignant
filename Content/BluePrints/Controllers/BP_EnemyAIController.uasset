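; Enemy AI controller that runs the BHT_Enemy_Base behavior tree and tracks the player as its target.
; AI Perception updates write the player to the TargetActor blackboard key when sensed, ignoring all other actors.
; Losing perception starts a short grace timer that empties the key, and sensing the player again cancels it so brief interruptions keep the target.
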(event `self.ReceiveBeginPlay`
  (`self.RunBehaviorTree` "/Game/BluePrints/NPCs/Enemies/TestEnemy/BHT_Enemy_Base.BHT_Enemy_Base"))

(event `self.AIPerception.OnTargetPerceptionUpdated`
  (params (Actor :type "Actor Object Reference") (Stimulus :type "AIStimulus Structure"))
  (set `self.SensedActor` Actor)
  (if (== Actor (`GameplayStatics.GetPlayerCharacter` 0))
    (if (`.bSuccessfullySensed` (break `AIStimulus` Stimulus))
      (`BlackboardComponent.SetValueAsObject` (`self.Blackboard`) "TargetActor" (`self.SensedActor`))
      (`KismetSystemLibrary.K2_ClearAndInvalidateTimerHandle` (`self.LoseTargetTimer`))
      (else
        (bind _returnvalue (`KismetSystemLibrary.K2_SetTimerDelegate` (delegate `LoseTarget`) 3.0)) ; Time for which player needs to be out of sight for enemy to stop chasing.
        (set `self.LoseTargetTimer` _returnvalue)))))

(event `LoseTarget`
  (`BlackboardComponent.SetValueAsObject` (`self.Blackboard`) "TargetActor" null))

(fn `UserConstructionScript`)