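; Configurable single hospital door prop for the morgue set, posed and styled entirely in the Construction Script with no runtime logic.
; Angle sets the door leaf's yaw, and WindowStyle shows one of four interior meshes: solid, long, medium or short window.
; Door, window frame and outer frame colors feed the CustomColor material parameter, using per-slot dynamic instances where medium and short inserts mix two colors.
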(fn `UserConstructionScript`
  (bind _doorcolor (`self.DoorColor`))
  (bind _sm_doorsingle_intframe3 (`self.SM_DoorSingle_IntFrame3`))
  (bind _windowframe_color (`self.WindowFrame Color`))
  (bind _sm_doorsingle_intframe2 (`self.SM_DoorSingle_IntFrame2`))
  (`SceneComponent.K2_SetRelativeRotation` (`self.SM_DoorSingle_DoorSingle`) (`KismetMathLibrary.MakeRotator` 0.0 0.0 (* (`self.Angle`) -1.0)) false false)
  (`MeshComponent.SetVectorParameterValueOnMaterials` (`self.SM_DoorSingle_DoorSingle`) "CustomColor" (`KismetMathLibrary.Conv_LinearColorToVector` _doorcolor))
  (`MeshComponent.SetVectorParameterValueOnMaterials` (`self.SM_DoorSingle_IntFrame0`) "CustomColor" (`KismetMathLibrary.Conv_LinearColorToVector` _doorcolor))
  (bind _returnvalue (`PrimitiveComponent.CreateDynamicMaterialInstance` (`self.SM_DoorSingle_IntFrame2`) 1 null "None"))
  (bind _returnvalue_2 (`PrimitiveComponent.CreateDynamicMaterialInstance` (`self.SM_DoorSingle_IntFrame1`) 1 null "None"))
  (`MaterialInstanceDynamic.SetVectorParameterValue` _returnvalue "CustomColor" _doorcolor)
  (`MaterialInstanceDynamic.SetVectorParameterValue` _returnvalue_2 "CustomColor" _doorcolor)
  (bind _returnvalue_3 (`PrimitiveComponent.CreateDynamicMaterialInstance` (`self.SM_DoorSingle_IntFrame1`) 0 null "None"))
  (bind _returnvalue_4 (`PrimitiveComponent.CreateDynamicMaterialInstance` (`self.SM_DoorSingle_IntFrame2`) 0 null "None"))
  (`MaterialInstanceDynamic.SetVectorParameterValue` _returnvalue_3 "CustomColor" _windowframe_color)
  (`MaterialInstanceDynamic.SetVectorParameterValue` _returnvalue_4 "CustomColor" _windowframe_color)
  (`MeshComponent.SetVectorParameterValueOnMaterials` (`self.SM_DoorSingle_IntFrame3`) "CustomColor" (`KismetMathLibrary.Conv_LinearColorToVector` _windowframe_color))
  (`MeshComponent.SetVectorParameterValueOnMaterials` (`self.SM_DoorSingle_Frame`) "CustomColor" (`KismetMathLibrary.Conv_LinearColorToVector` (`self.Frame Color`)))
  (switch `/Game/Mortuary_Content/Horror_Collection_Morgue/Materials/E_Door_Windows_Enum` (`self.WindowStyle`)
    (:`NewEnumerator0`
      (`SceneComponent.SetVisibility` _sm_doorsingle_intframe3 false true)
      (`SceneComponent.SetVisibility` _sm_doorsingle_intframe2 false true)
      (`SceneComponent.SetVisibility` (`self.SM_DoorSingle_IntFrame1`) false true)
      (`SceneComponent.SetVisibility` (`self.SM_DoorSingle_IntFrame0`) true true))
    (:`NewEnumerator1`
      (`SceneComponent.SetVisibility` _sm_doorsingle_intframe2 false true)
      (`SceneComponent.SetVisibility` (`self.SM_DoorSingle_IntFrame1`) false true)
      (`SceneComponent.SetVisibility` (`self.SM_DoorSingle_IntFrame0`) false true)
      (`SceneComponent.SetVisibility` _sm_doorsingle_intframe3 true true))
    (:`NewEnumerator2`
      (`SceneComponent.SetVisibility` _sm_doorsingle_intframe3 false true)
      (`SceneComponent.SetVisibility` (`self.SM_DoorSingle_IntFrame1`) false true)
      (`SceneComponent.SetVisibility` (`self.SM_DoorSingle_IntFrame0`) false true)
      (`SceneComponent.SetVisibility` _sm_doorsingle_intframe2 true true))
    (:`NewEnumerator3`
      (`SceneComponent.SetVisibility` _sm_doorsingle_intframe3 false true)
      (`SceneComponent.SetVisibility` _sm_doorsingle_intframe2 false true)
      (`SceneComponent.SetVisibility` (`self.SM_DoorSingle_IntFrame0`) false true)
      (`SceneComponent.SetVisibility` (`self.SM_DoorSingle_IntFrame1`) true true))))