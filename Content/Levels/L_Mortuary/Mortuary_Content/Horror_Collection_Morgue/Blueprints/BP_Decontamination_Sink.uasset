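; Decontamination sink prop for the morgue level, with four cabinet doors, three taps and three pairs of tap arms that can be posed per instance.
; The Construction Script passes each yaw variable to a shared RotateZ helper, which sets that mesh's relative rotation.
; An invert flag negates the angle for two of the doors and the right-hand arms so they mirror their counterparts.
; It has no active runtime logic.
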(fn `RotateZ`
  (params (`Z (Yaw)` :type "Float (double-precision)") (InvertZ :type Boolean) (TargetMesh :type "SceneComponent Object Reference"))
  (if InvertZ
    (`SceneComponent.K2_SetRelativeRotation` TargetMesh (`KismetMathLibrary.MakeRotator` 0.0 0.0 (* `Z (Yaw)` -1.0)) false false)
    (else
      (`SceneComponent.K2_SetRelativeRotation` TargetMesh (`KismetMathLibrary.MakeRotator` 0.0 0.0 `Z (Yaw)`) false false)))
  (return))

(fn `UserConstructionScript`
  (`self.RotateZ` (`self.OpenDoor_1st`) false (`self.SM_Sink_Door1`))
  (`self.RotateZ` (`self.OpenDoor_2nd`) false (`self.SM_Sink_Door2`))
  (`self.RotateZ` (`self.OpenDoor_3rd`) true (`self.SM_Sink_Door3`))
  (`self.RotateZ` (`self.OpenDoor_4th`) true (`self.SM_Sink_Door4`))
  (`self.RotateZ` (`self.Tap_1st`) false (`self.StaticMesh4`))
  (`self.RotateZ` (`self.Tap_2nd`) false (`self.StaticMesh1`))
  (`self.RotateZ` (`self.Tap_3rd`) false (`self.SM_Sink_T03_low`))
  (`self.RotateZ` (`self.Arm_1st_L`) false (`self.StaticMesh5`))
  (`self.RotateZ` (`self.Arm_1st_R`) true (`self.StaticMesh3`))
  (`self.RotateZ` (`self.Arm_2nd_L`) false (`self.StaticMesh`))
  (`self.RotateZ` (`self.Arm_2nd_R`) true (`self.StaticMesh2`))
  (`self.RotateZ` (`self.Arm_3rd_L`) false (`self.SM_Sink_T06_low`))
  (`self.RotateZ` (`self.Arm_3rd_R`) true (`self.SM_Sink_T04_low`)))